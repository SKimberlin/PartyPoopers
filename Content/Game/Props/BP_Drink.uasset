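; Drink prop actor that spills its contents when tipped over or moved quickly.
; Each Tick turns the Niagara effect on while roll or pitch passes 90 degrees or velocity exceeds a threshold, and off otherwise.
; While spilling, a Delay on Tick throttles spawning of BP_WineCollision actors at the Arrow component's transform to roughly one every half second.
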(event `self.ReceiveTick`
  (params (DeltaSeconds :type "Float (single-precision)"))
  (bind _returnvalue (or (or (> (`KismetMathLibrary.Abs` (.roll (`self.K2_GetActorRotation`))) 90.0) (> (`KismetMathLibrary.Abs` (.pitch (`self.K2_GetActorRotation`))) 90.0)) (> (`KismetMathLibrary.VSize` (`self.GetVelocity`)) 150.0)))
  (`ActorComponent.SetActive` (`self.Niagara`) _returnvalue false)
  (if _returnvalue
    (`KismetSystemLibrary.Delay` 0.5)
    (bind _returnvalue_2 (`|SpawnActorFromClass` "/Game/Game/Props/BP_WineCollision.BP_WineCollision_C" (`SceneComponent.K2_GetComponentToWorld` (`self.Arrow`)) "Undefined" "MultiplyWithRoot" self null))
    (`/Engine/EditorBlueprintResources/StandardMacros.IsValid` _returnvalue_2)))

(fn `UserConstructionScript`)