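; BP_TestGameInstance is a test game instance that handles LAN multiplayer sessions and switching between main menu and gameplay input.
; CreateMPSession creates a two-slot LAN session and opens TestWorld as a listen server, while JoinMPSession joins a supplied search result; both print errors on failure.
; UIShowMainMenu lazily creates and caches WB_StartMenu, then shows it with UI-only input and a cursor.
; PlayerStart restores game-only input and hides the cursor.
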(event `CreateMPSession`
  (`CreateSessionCallbackProxy.CreateSession` (`GameplayStatics.GetPlayerController` 0) 2 true
    (:`OnSuccess`
      (`GameplayStatics.OpenLevelBySoftObjectPtr` "/Game/Game/TestingCollin/TestWorld.TestWorld" true "listen"))
    (:`OnFailure`
      (`KismetSystemLibrary.PrintString` "Error: Failed to create session!" true true (struct :`R` 0.328125 :`G` 0.016917 :`B` 0.013653 :`A` 1.0)))))

(event `JoinMPSession`
  (params (SessionResult :type "BlueprintSessionResult Structure"))
  (`JoinSessionCallbackProxy.JoinSession` (`GameplayStatics.GetPlayerController` 0) SessionResult
    (:`OnFailure`
      (`KismetSystemLibrary.PrintString` "Error: Failed to join session!" true true (struct :`R` 0.328125 :`G` 0.016917 :`B` 0.013653 :`A` 1.0)))))

(fn `PlayerStart`
  (`WidgetBlueprintLibrary.SetInputMode_GameOnly` (`GameplayStatics.GetPlayerController` 0))
  (set `PlayerController.bShowMouseCursor` false (`GameplayStatics.GetPlayerController` 0)))

(fn `UIShowMainMenu`
  (`/Engine/EditorBlueprintResources/StandardMacros.IsValid` (`self.WBMainMenu`)
    (:`Is Valid`
      _)
    (:`Is Not Valid`
      (bind _returnvalue (`|CreateWidget` "/Game/Game/TestingCollin/WB_StartMenu.WB_StartMenu_C" (`GameplayStatics.GetPlayerController` 0)))
      (set `self.WBMainMenu` _returnvalue)))
  (`UserWidget.AddToViewport` (`self.WBMainMenu`) 0)
  (`WidgetBlueprintLibrary.SetInputMode_UIOnlyEx` (`GameplayStatics.GetPlayerController` 0) (`self.WBMainMenu`))
  (set `PlayerController.bShowMouseCursor` true (`GameplayStatics.GetPlayerController` 0))
  (return))