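; BP_Mask is a cosmetic mask actor that gives a guest character a randomized mask.
; On BeginPlay it picks a random mesh, then casts its Instigator to BP_Guest and stops if that fails.
; It then snaps to the MaskSocket on the guest's mesh, keeping relative scale, and applies a random material to the first slot.
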(event `self.ReceiveBeginPlay`
  (`StaticMeshComponent.SetStaticMesh` (`self.StaticMesh`) (`KismetArrayLibrary.Array_Random` (`self.MaskMeshes`)))
  (bind _asbp_guest (cast `/Game/Game/TestingSeth/Guest/Blueprints/BP_Guest` (`self.GetInstigator`)))
  (`self.K2_AttachToComponent` (`Character.Mesh` _asbp_guest) "MaskSocket" "SnapToTarget" "SnapToTarget" "KeepRelative")
  (`PrimitiveComponent.SetMaterial` (`self.StaticMesh`) 0 (`KismetArrayLibrary.Array_Random` (`self.Materials`))))

(fn `UserConstructionScript`)