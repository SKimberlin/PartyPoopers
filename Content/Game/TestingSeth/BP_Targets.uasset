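; BP_Targets is a test Blueprint that picks a random BP_Guest as a target and shows its mask for debugging.
; BeginPlay stores the chosen guest as the sole entry in Targets and starts a five-second timer bound to the Target event, which is currently empty.
; Tick prints the first target's Mask enum as a string every frame.
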(event `self.ReceiveBeginPlay`
  (bind _outactors (`GameplayStatics.GetAllActorsOfClass` "/Game/Game/TestingSeth/Guest/Blueprints/BP_Guest.BP_Guest_C"))
  (set `self.Targets` (`|MakeArray` (`KismetArrayLibrary.Array_Random` _outactors)))
  (`KismetSystemLibrary.K2_SetTimerDelegate` (delegate `Target`) 5.0))

(event `Target`)

(event `self.ReceiveTick`
  (params (DeltaSeconds :type "Float (single-precision)"))
  (`KismetSystemLibrary.PrintString` (`|GetEnumeratorNameAsString` (`/Game/Game/TestingSeth/Guest/Blueprints/BP_Guest.Mask` (`|GetArrayItem` (`self.Targets`))))))

(fn `UserConstructionScript`)