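; BP_Dossier is an actor that presents a target dossier through a widget component.
; SetVisible and SetHidden toggle the actor's visibility together with the widget's collision, switching between query-only and none.
; SetTargetData casts the component's widget to WBP_Dossier and copies the supplied target data into it.
; The event graph and construction script are empty, so these functions rely on external callers.
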(event `self.ReceiveBeginPlay`)

(fn `SetHidden`
  (`self.SetActorHiddenInGame` true)
  (`PrimitiveComponent.SetCollisionEnabled` (`self.Widget`) "NoCollision"))

(fn `SetTargetData`
  (params (TargetData :type "Array of /Game/Game/TestingSeth/F_TargetData Structure"))
  (bind _aswbp_dossier (cast `/Game/Game/TestingSeth/WBP_Dossier` (`WidgetComponent.GetWidget` (`self.Widget`))))
  (set `/Game/Game/TestingSeth/WBP_Dossier.TargetData` TargetData _aswbp_dossier))

(fn `SetVisible`
  (`self.SetActorHiddenInGame` false)
  (`PrimitiveComponent.SetCollisionEnabled` (`self.Widget`) "QueryOnly"))

(fn `UserConstructionScript`)