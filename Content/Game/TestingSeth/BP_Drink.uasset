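; BP_Drink is a drink actor that drives a Niagara effect, likely spilling liquid, from its orientation and motion.
; Every Tick it activates the Niagara component when absolute roll or pitch passes 90 degrees or speed exceeds a threshold, and deactivates it otherwise.
; The activation does not reset the system, and the actor has no other active logic.
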(event `self.ReceiveTick`
  (params (DeltaSeconds :type "Float (single-precision)"))
  (`ActorComponent.SetActive` (`self.Niagara`) (or (or (> (`KismetMathLibrary.Abs` (.roll (`self.K2_GetActorRotation`))) 90.0) (> (`KismetMathLibrary.Abs` (.pitch (`self.K2_GetActorRotation`))) 90.0)) (> (`KismetMathLibrary.VSize` (`self.GetVelocity`)) 150.0)) false))

(fn `UserConstructionScript`)