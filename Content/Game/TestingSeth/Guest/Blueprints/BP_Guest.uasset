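; BP_Guest is an AI-driven guest character with health and a randomized masked appearance.
; On BeginPlay it picks random skin, shirt and suit materials, then attaches a random bird, wolf or bunny mask to a head mesh socket.
; A one-shot timer sets a bathroom blackboard key on its Guest_Controller and restarts BT_Guest.
; Damage drains health, and at zero the mesh simulates physics and the movement component is destroyed.
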(event `self.ReceiveBeginPlay`
  (bind _maskmesh (`self.MaskMesh`))
  (bind _mesh (`self.Mesh`))
  (`|ExecutionSequence`
    (:`then_0`
      (set `self.Health` (`self.MaxHealth`))
      (set `self.Mask` (cast `/Game/Game/TestingSeth/EMasks` (`KismetMathLibrary.Conv_IntToByte` (`KismetMathLibrary.RandomIntegerInRange` 0 2)))))
    (:`then_1`
      (`|ExecutionSequence`
        (:`then_0`
          (`PrimitiveComponent.SetMaterial` _mesh 0 (`KismetArrayLibrary.Array_Random` (`self.SkinMaterials`))))
        (:`then_1`
          (`PrimitiveComponent.SetMaterial` _mesh 1 (`KismetArrayLibrary.Array_Random` (`self.ShirtMaterials`))))
        (:`then_2`
          (`PrimitiveComponent.SetMaterial` _mesh 2 (`KismetArrayLibrary.Array_Random` (`self.SuitMaterials`))))))
    (:`then_2`
      (`SceneComponent.K2_AttachToComponent` (`self.MaskMesh`) (`self.Mesh`) "MaskSocket" "SnapToTarget" "SnapToTarget" "KeepRelative" true)
      (switch `/Game/Game/TestingSeth/EMasks` (`self.Mask`)
        (:`NewEnumerator0`
          (`StaticMeshComponent.SetStaticMesh` _maskmesh "/Game/Game/TestingSeth/Masks_BirdMask.Masks_BirdMask"))
        (:`NewEnumerator1`
          (`StaticMeshComponent.SetStaticMesh` _maskmesh "/Game/Game/TestingSeth/Masks_WolfMask.Masks_WolfMask"))
        (:`NewEnumerator2`
          (`StaticMeshComponent.SetStaticMesh` _maskmesh "/Game/Game/TestingSeth/Masks_BunnyMask.Masks_BunnyMask")))
      (`PrimitiveComponent.SetMaterial` (`self.MaskMesh`) 0 (`KismetArrayLibrary.Array_Random` (`self.MaskMaterials`)))
      (`KismetSystemLibrary.K2_SetTimerDelegate` (delegate `Bathroom`) 5.0))))

(event `self.ReceiveAnyDamage`
  (params (Damage :type "Float (single-precision)") (DamageType :type "DamageType Object Reference") (InstigatedBy :type "Controller Object Reference") (DamageCauser :type "Actor Object Reference"))
  (bind _output_get (set `self.Health` (- (`self.Health`) Damage)))
  (if (<= _output_get 0.0)
    (`PrimitiveComponent.SetSimulatePhysics` (`self.Mesh`) true)
    (`ActorComponent.K2_DestroyComponent` (`self.CharacterMovement`))))

(event `Bathroom`
  (bind _asguest_controller (cast `/Game/Game/TestingSeth/Guest/Blueprints/AI/Guest_Controller` (`self.GetController`)))
  (`BrainComponent.StopLogic` (`AIController.BrainComponent` _asguest_controller) "")
  (`BlackboardComponent.SetValueAsBool` (`AIBlueprintHelperLibrary.GetBlackboard` _asguest_controller) (`self.BathroomKey`) true)
  (`AIController.RunBehaviorTree` _asguest_controller "/Game/Game/TestingSeth/Guest/Blueprints/AI/BT_Guest.BT_Guest"))

(fn `UserConstructionScript`)