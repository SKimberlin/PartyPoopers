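; BP_Spawner is an actor that populates the area around itself with BP_Guest actors.
; Its SpawnGuests event first destroys every existing BP_Guest in the world, then spawns GuestAmount new ones.
; Each guest is placed at a random navigable point within SpawnRadius of the spawner, with collision adjustment that skips spawns still colliding.
; Nothing in this Blueprint calls SpawnGuests, as BeginPlay and Tick are empty.
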(event `self.ReceiveBeginPlay`)

(event `SpawnGuests`
  (bind _outactors (`GameplayStatics.GetAllActorsOfClass` "/Game/Game/Characters/Guest/Blueprints/BP_Guest.BP_Guest_C"))
  (for _array_element _outactors
    (`self.K2_DestroyActor` _array_element))
  (for _ (range (`self.GuestAmount`))
    (bind _randomlocation (`NavigationSystemV1.K2_GetRandomLocationInNavigableRadius` (`NavigationSystemV1.GetNavigationSystem`) (`self.K2_GetActorLocation`) (`self.SpawnRadius`) null null))
    (`|SpawnActorFromClass` "/Game/Game/Characters/Guest/Blueprints/BP_Guest.BP_Guest_C" (`KismetMathLibrary.Conv_VectorToTransform` _randomlocation) "AdjustIfPossibleButDontSpawnIfColliding" "MultiplyWithRoot" null null)))

(fn `UserConstructionScript`)