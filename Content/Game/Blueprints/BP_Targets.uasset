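; BP_Targets picks one random BP_Guest in the level as the target and reports on it through debug prints.
; At BeginPlay it stores that guest in Targets, then a five-second timer prints the guest's mask enum and the name of its mask mesh material.
; Tick polls the target's health and prints a death message every frame it is at or below zero.
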(event `self.ReceiveBeginPlay`
  (bind _outactors (`GameplayStatics.GetAllActorsOfClass` "/Game/Game/Characters/Guest/Blueprints/BP_Guest.BP_Guest_C"))
  (set `self.Targets` (`|MakeArray` (`KismetArrayLibrary.Array_Random` _outactors)))
  (`KismetSystemLibrary.K2_SetTimerDelegate` (delegate `Target`) 5.0))

(event `Target`
  (bind _output (`|GetArrayItem` (`self.Targets`)))
  (`KismetSystemLibrary.PrintString` (`|GetEnumeratorNameAsString` (`/Game/Game/Characters/Guest/Blueprints/BP_Guest.Mask` _output)))
  (`KismetSystemLibrary.PrintString` (`KismetSystemLibrary.GetDisplayName` (`PrimitiveComponent.GetMaterial` (`/Game/Game/Characters/Guest/Blueprints/BP_Guest.MaskMesh` _output) 0))))

(event `self.ReceiveTick`
  (params (DeltaSeconds :type "Float (single-precision)"))
  (if (<= (`/Game/Game/Characters/Guest/Blueprints/BP_Guest.Health` (`|GetArrayItem` (`self.Targets`))) 0.0)
    (`KismetSystemLibrary.PrintString` "Target Dead")))

(fn `UserConstructionScript`)