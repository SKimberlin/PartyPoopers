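; BP_SniperRifle is a weapon child Blueprint that adds a scope overlay, adjustable zoom and scoped hitscan shooting.
; It creates WB_Scope on BeginPlay, and Aim toggles it while setting the character camera's FOV and scaling sensitivity to match.
; AdjustAim changes the clamped FOV, applying it live during ADS.
; Shoot, only in ADS, line-traces from the camera toward forward vector times Range (not offset by start), applies damage and prints the hit actor.
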(event `self.ReceiveBeginPlay`
  (`parent.ReceiveBeginPlay`)
  (bind _returnvalue (`|CreateWidget` "/Game/Game/UI/WB_Scope.WB_Scope_C"))
  (bind _output_get (set `self.ScopeWB` _returnvalue))
  (`UserWidget.AddToViewport` _output_get 0))

(fn `AdjustAim`
  (params (Value :type "Float (double-precision)"))
  (`parent.AdjustAim` Value)
  (set `self.FOV` (`KismetMathLibrary.FClamp` (+ (* Value -3.0) (`self.FOV`)) 0.1 70.0))
  (bind _asbp_first_person_character (cast `/Game/FirstPerson/Blueprints/BP_FirstPersonCharacter` (`self.Character`)))
  (if (`/Game/FirstPerson/Blueprints/BP_FirstPersonCharacter.ADS` _asbp_first_person_character)
    (`CameraComponent.SetFieldOfView` (`/Game/FirstPerson/Blueprints/BP_FirstPersonCharacter.FirstPersonCamera` _asbp_first_person_character) (`self.FOV`))))

(fn `Aim`
  (params (Aiming :type Boolean))
  (`parent.Aim` Aiming)
  (set `/Game/Game/UI/WB_Scope.IsActive` Aiming (`self.ScopeWB`))
  (if Aiming
    (bind _asbp_first_person_character (cast `/Game/FirstPerson/Blueprints/BP_FirstPersonCharacter` (`self.Character`)))
    (`CameraComponent.SetFieldOfView` (`/Game/FirstPerson/Blueprints/BP_FirstPersonCharacter.FirstPersonCamera` _asbp_first_person_character) (`self.FOV`))
    (set `/Game/FirstPerson/Blueprints/BP_FirstPersonCharacter.Sensitivity` (/ (`self.FOV`) 80.0) _asbp_first_person_character)
    (else
      (bind _asbp_first_person_character_2 (cast `/Game/FirstPerson/Blueprints/BP_FirstPersonCharacter` (`self.Character`)))
      (`CameraComponent.SetFieldOfView` (`/Game/FirstPerson/Blueprints/BP_FirstPersonCharacter.FirstPersonCamera` _asbp_first_person_character_2) 90.0)
      (set `/Game/FirstPerson/Blueprints/BP_FirstPersonCharacter.Sensitivity` 1.0 _asbp_first_person_character_2))))

(fn `Shoot`
  (bind _asbp_first_person_character (cast `/Game/FirstPerson/Blueprints/BP_FirstPersonCharacter` (`self.Character`) :!pure true))
  (bind _firstpersoncamera (`/Game/FirstPerson/Blueprints/BP_FirstPersonCharacter.FirstPersonCamera` _asbp_first_person_character))
  (`parent.Shoot`)
  (if (`/Game/FirstPerson/Blueprints/BP_FirstPersonCharacter.ADS` _asbp_first_person_character)
    (bind _outhit (`KismetSystemLibrary.LineTraceSingle` (`SceneComponent.K2_GetComponentLocation` _firstpersoncamera) (+ (* (`SceneComponent.GetForwardVector` _firstpersoncamera) (`self.Range`)) (0.0 0.0 0.0)) "TraceTypeQuery1" false (`|MakeArray` (`GameplayStatics.GetPlayerPawn` 0) :!type "Actor Object Reference") "ForDuration" true (struct :`R` 1.0 :`A` 1.0) (struct :`G` 1.0 :`A` 1.0) 1.0))
    (`GameplayStatics.ApplyDamage` (`.HitActor` (`GameplayStatics.BreakHitResult` _outhit)) (`self.Damage`) null (`self.Character`))
    (`KismetSystemLibrary.PrintString` (`KismetSystemLibrary.GetDisplayName` (`.HitActor` (`GameplayStatics.BreakHitResult` _outhit))))))

(fn `UserConstructionScript`
  (`parent.UserConstructionScript`))